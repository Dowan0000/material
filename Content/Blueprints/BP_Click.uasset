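; BP_Click is a clickable cube actor that builds up with each click until it explodes.
; On BeginPlay it creates a dynamic material instance for the cube.
; Each click plays a sound and sets the emissive parameter, using one rising counter for both pitch and glow.
; Past a threshold it spawns an explosion effect and sound, then destroys itself; several leftover nodes, including color setting, are unconnected.
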(event OnClicked(Cube)
  (params (TouchedComponent :type Primitive%20Component%20Object%20Reference) (ButtonPressed :type Key%20Structure :default "None"))
  (Audio|PlaySound2D "/Engine/VREditor/Sounds/VR_click1_Cue.VR_click1_Cue" 1.0 (Variables|Default|GetValue_0) 0.0 0 0)
  (Rendering|Material|SetScalarParameterValue (Variables|Default|GetEmi) "Emissive" (Variables|Default|GetValue_0) :!class /Script/Engine.MaterialInstanceDynamic)
  (Variables|Default|SetValue_0 (+ (Variables|Default|GetValue_0) 0.2))
  (if (> (Variables|Default|GetValue_0) 1.5)
    (Effects|SpawnEmitteratLocation "/Game/StarterContent/Particles/P_Explosion.P_Explosion" (Transformation|GetWorldLocation (Variables|Default|GetCube)))
    (Audio|PlaySound2D "/Game/StarterContent/Audio/Explosion_Cue.Explosion_Cue" 1.0 1.0 0.0 0 0)
    (Actor|DestroyActor)))

(event EventBeginPlay
  (bind _returnvalue (Rendering|Material|CreateDynamicMaterialInstance (Variables|Default|GetCube) 0 0 "None" :!class /Script/Engine.PrimitiveComponent))
  (Variables|Default|SetEmi _returnvalue))

(fn ConstructionScript)